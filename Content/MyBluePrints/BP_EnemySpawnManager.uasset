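; BP_EnemySpawnManager is a wave manager that starts a new enemy wave once no BP_Enemy actors remain in the level.
; NewEnemyWaveCheck takes a transform, counts living enemies and, when none remain, calls SpawnNewEnemies and spawns a BP_Key at that transform.
; SpawnNewEnemies waits a short delay, then tells every BP_EnemySpawner found through GetAllActorsOfClass to spawn an enemy.
; Debug prints report spawner count and wave progress.
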(event Custom|NewEnemyWaveCheck
  (params (Transform :type Transform))
  (Development|PrintString "checking enemy count" true true "(R=1.000000,G=0.013110,B=0.000000,A=1.000000)")
  (bind _outactors (Actor|GetAllActorsOfClass "/Game/MyBluePrints/BP_Enemy.BP_Enemy_C"))
  (if (> (Utilities|Array|Length _outactors) 0)
    (Development|PrintString "There are still more enemies in the level")
    (else
      (CallFunction|SpawnNewEnemies)
      (Game|SpawnActorfromClass "/Game/MyBluePrints/BP_Key.BP_Key_C" Transform "Undefined" "MultiplyWithRoot" 0 0))))

(event Custom|Spawn%20New%20Enemies
  (Development|PrintString "Spawning new enemies in 3 seconds")
  (Utilities|FlowControl|Delay 3.0)
  (bind _outactors (Actor|GetAllActorsOfClass "/Game/MyBluePrints/BP_EnemySpawner.BP_EnemySpawner_C"))
  (for (_array_element _array_index) _outactors
    (Default|SpawnNewEnemy _array_element)
    (Development|PrintString (Utilities|String|Append (Utilities|String|ToString(Integer) _array_index) ". " (Utilities|GetDisplayName _array_element) " is Spawning...") true true (Utilities|Struct|MakeLinearColor (Math|Random|RandomFloatinRange 0.1 1.0) (Math|Random|RandomFloatinRange 0.1 1.0) (Math|Random|RandomFloatinRange 0.1 1.0) 1.0)))
  (Development|PrintString "new wave complete"))

(event EventBeginPlay
  (Development|PrintString "Spawn Manger is live")
  (bind _outactors (Actor|GetAllActorsOfClass "/Game/MyBluePrints/BP_EnemySpawner.BP_EnemySpawner_C"))
  (Development|PrintString (Utilities|String|Append "there are " (Utilities|String|ToString(Integer) (Utilities|Array|Length _outactors)) " spawners in the level." "there are " "##" "enemies in the level.") true true "(R=1.000000,G=0.000000,B=0.928120,A=1.000000)"))

(fn ConstructionScript)