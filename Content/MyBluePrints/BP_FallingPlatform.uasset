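; Falling platform actor that drops after the third-person character steps on it, then returns to its starting place.
; A box overlap, gated by a Ready flag, starts a delay before enabling physics on the platform mesh.
; After a second delay, physics stops and a timeline lerps it back to the transform saved at BeginPlay, re-arming it.
; Material swaps mark each state; the explosion sound nodes never run.
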(event OnComponentBeginOverlap(Box)
  (params (OverlappedComponent :type Primitive%20Component%20Object%20Reference) (OtherActor :type Actor%20Object%20Reference) (OtherComp :type Primitive%20Component%20Object%20Reference) (OtherBodyIndex :type Integer) (bFromSweep :type Boolean) (SweepResult :type Hit%20Result%20Structure%20%28by%20ref%29))
  (Development|PrintString "something is standing on mme")
  (if (Variables|Default|GetReady)
    (Utilities|Casting|CastToBP_ThirdPersonCharacter OtherActor)
    (CallFunction|Activate)))

(event Custom|Activate
  (Variables|Default|SetReady false)
  (Rendering|Material|SetMaterial (Variables|Default|GetPlatform) 0 "/Game/MyMaterials/FallingPlatformMats/MI_ActivePlatform.MI_ActivePlatform")
  (Development|PrintString "starting count down")
  (Utilities|FlowControl|Delay (Variables|PlatformSettings|GetFallDelayDuration))
  (CallFunction|Falling))

(event Custom|Falling
  (bind _platform (Variables|Default|GetPlatform))
  (Development|PrintString "Curently falling")
  (Rendering|Material|SetMaterial _platform 0 "/Game/MyMaterials/FallingPlatformMats/MI_FallingPlatform.MI_FallingPlatform")
  (Physics|SetSimulatePhysics _platform true)
  (Utilities|FlowControl|Delay (Variables|PlatformSettings|GetResetDelayDuration))
  (CallFunction|Reset))

(event Custom|Reset
  (bind _platform (Variables|Default|GetPlatform))
  (Development|PrintString "Reseting")
  (Rendering|Material|SetMaterial _platform 0 "/Game/MyMaterials/FallingPlatformMats/MI_ResetingPLatform.MI_ResetingPLatform")
  (Physics|SetSimulatePhysics _platform false)
  (Variables|Default|SetFallenTransform (Transformation|GetWorldTransform _platform))
  (bind _newtrack_0 (Timeline|ResetToStartTransform PlayFromStart)
    (:Update
      (Transformation|SetWorldTransform (Variables|Default|GetPlatform) (Math|Transform|Lerp(Transform) (Variables|Default|GetFallenTransform) (Variables|Default|GetStarting%20Tansform) _newtrack_0) false false))
    (:Finished
      (Variables|Default|SetReady true)
      (Rendering|Material|SetMaterial (Variables|Default|GetPlatform) 0 "/Game/MyMaterials/FallingPlatformMats/MI_FallinngPlatReady.MI_FallinngPlatReady"))))

(event EventBeginPlay
  (Variables|Default|SetStarting%20Tansform (Transformation|GetWorldTransform (Variables|Default|GetPlatform))))

(event Collision|EventActorBeginOverlap
  (params (OtherActor :type Actor%20Object%20Reference)))

(event EventTick
  (params (DeltaSeconds :type Float%20%28single-precision%29)))

(fn ConstructionScript)