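; Elevator actor whose platform moves along a timeline when something begins overlapping its trigger box.
; The timeline's float track lerps the platform's location and rotation between the Start and End component transforms.
; Timeline event tracks swap the platform material to show moving and stopped states.
; A Ready flag blocks retriggering until the timeline finishes, which restores the ready material.
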(event OnComponentBeginOverlap(Box)
  (params (OverlappedComponent :type Primitive%20Component%20Object%20Reference) (OtherActor :type Actor%20Object%20Reference) (OtherComp :type Primitive%20Component%20Object%20Reference) (OtherBodyIndex :type Integer) (bFromSweep :type Boolean) (SweepResult :type Hit%20Result%20Structure%20%28by%20ref%29))
  (bind _platform (Variables|Default|GetPlatform))
  (if (Variables|Default|GetReady)
    (Variables|Default|SetReady false)
    (bind _newtrack_0 (Timeline|Timeline PlayFromStart)
      (:Update
        (Transformation|SetWorldLocationAndRotation (Variables|Default|GetPlatform) (.location (Math|Transform|Lerp(Transform) (Transformation|GetWorldTransform (Variables|Default|GetStart)) (Transformation|GetWorldTransform (Variables|Default|GetEnd)) _newtrack_0)) (.rotation (Math|Transform|Lerp(Transform) (Transformation|GetWorldTransform (Variables|Default|GetStart)) (Transformation|GetWorldTransform (Variables|Default|GetEnd)) _newtrack_0)) false false))
      (:Finished
        (Rendering|Material|SetMaterial _platform 0 "/Game/MyMaterials/FallingPlatformMats/MI_FallinngPlatReady.MI_FallinngPlatReady")
        (Variables|Default|SetReady true))
      (:MOving
        (Rendering|Material|SetMaterial _platform 0 "/Game/MyMaterials/FallingPlatformMats/MI_ActivePlatform.MI_ActivePlatform"))
      (:Stoped
        (Rendering|Material|SetMaterial _platform 0 "/Game/MyMaterials/FallingPlatformMats/MI_FallingPlatform.MI_FallingPlatform")))))

(event EventBeginPlay)

(event Collision|EventActorBeginOverlap
  (params (OtherActor :type Actor%20Object%20Reference)))

(event EventTick
  (params (DeltaSeconds :type Float%20%28single-precision%29)))

(fn ConstructionScript)